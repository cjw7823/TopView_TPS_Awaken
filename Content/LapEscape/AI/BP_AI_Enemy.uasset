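; AI enemy character for LapEscape that melee-attacks player characters and rewards gold when killed.
; An OnAttack-guarded montage plays on request or IsClose RepNotify, while DoAttack box-traces forward and applies damage once per trace through a server request event.
; Incoming damage updates BPStateComponent; death sets the blackboard IsDie key and plays a montage.
; Tick then handles delayed destruction, adds bonus gold to the GameState and randomly spawns a heal orb.
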(event `self.ReceiveBeginPlay`
  ;[1 1 1] 생성시 이동속도 조절
  (set `CharacterMovementComponent.MaxWalkSpeed` (`KismetMathLibrary.RandomFloatInRange` 800.0 800.0) (`self.CharacterMovement`))
  (`self.SpawnDefaultController`))

(event `ReqApplyDamage`
  (params (DamagedActor :type "Actor Object Reference (by ref)") (BaseDamage :type "Float (double-precision)") (EventInstigator :type "Controller Object Reference (by ref)") (DamageCauser :type "Actor Object Reference (by ref)") (`Hit Location` :type "Vector Structure") (`Impulse Dir` :type "Vector Structure"))
  ;[1 0 0] (Server)Apply Damage
  (`GameplayStatics.ApplyDamage` DamagedActor BaseDamage EventInstigator DamageCauser))

(event `self.ReceiveAnyDamage`
  (params (Damage :type "Float (single-precision)") (DamageType :type "DamageType Object Reference") (InstigatedBy :type "Controller Object Reference") (DamageCauser :type "Actor Object Reference"))
  ;[1 0 0] (Server)Any Damage 요청
  (bind _isdeath (`/Game/LapEscape/AI/BP_StateComponent.SetHP` (`self.BP_StateComponent`) Damage))
  (if _isdeath
    (`BlackboardComponent.SetValueAsBool` (`AIBlueprintHelperLibrary.GetBlackboard` null) "IsDie" true)
    (`self.ResDeathMontage`)))

(event `ResDeathMontage`
  ;[1 1 1] Death Montage
  (if (not (`/Game/LapEscape/AI/BP_StateComponent.IsDeath` (`self.BP_StateComponent`)))
    (`self.PlayAnimMontage` "/Game/Mannequin/AI_Character/Anim/Death_1_Montage.Death_1_Montage")
    (set `/Game/LapEscape/AI/BP_StateComponent.IsDeath` true (`self.BP_StateComponent`))))

(event `self.ReceiveTick`
  (params (DeltaSeconds :type "Float (single-precision)"))
  ;[1 1 1] 죽으면 소멸
  (if (`/Game/LapEscape/AI/BP_StateComponent.IsDeath` (`self.BP_StateComponent`))
    (`KismetSystemLibrary.Delay` 3.0)
    (`self.K2_DestroyActor`)
    (bind _asbp_my_game_state (cast `/Game/LapEscape/GameMode/BP_MyGameState` (`GameplayStatics.GetGameState`)))
    (set `/Game/LapEscape/GameMode/BP_MyGameState.Gold` (+ (`/Game/LapEscape/GameMode/BP_MyGameState.Gold` _asbp_my_game_state) (`/Game/LapEscape/GameMode/BP_MyGameState.BonusGold` _asbp_my_game_state)) _asbp_my_game_state)
    ;[1 1 1] 30%확률로 체력 구슬 드랍
    (if (>= (`KismetMathLibrary.RandomInteger` 11) 7)
      (`|SpawnActorFromClass` "/Game/LapEscape/Blueprints/BP_HealActor.BP_HealActor_C" (`self.GetTransform`) "Undefined" "OverrideRootScale" null null))))

(event `ResAttackMontage`
  ;[1 1 1] Attack Montage
  (`self.AttackMontage`))

(fn `AttackMontage`
  (if (not (`self.OnAttack`))
    (`self.PlayAnimMontage` "/Game/Mannequin/AI_Character/Anim/Attack_Anim_Montage.Attack_Anim_Montage" 1.5)
    (set `self.OnAttack` true)))

(fn `DoAttack`
  (locals (OnceAttack :type Boolean :default true))
  (bind _returnvalue (`self.K2_GetActorLocation`))
  (bind (_outhits _returnvalue_2) (`KismetSystemLibrary.BoxTraceMultiForObjects` :`Start` _returnvalue :`End` (+ _returnvalue (* (`self.GetActorForwardVector`) 250.0)) :`ObjectTypes` (`|MakeArray` "ObjectTypeQuery1" "ObjectTypeQuery2" "ObjectTypeQuery3" "ObjectTypeQuery4" "ObjectTypeQuery6" :!type "EObjectTypeQuery Enum") :`DrawDebugType` "ForDuration"))
  (if _returnvalue_2
    (for _array_element _outhits
      (bind _asbp_mixamo_character (cast `/Game/LapEscape/GameMode/BP_MixamoCharacter` (`.HitActor` (`GameplayStatics.BreakHitResult` _array_element))))
      (if (`local.OnceAttack`)
        (set `local.OnceAttack` false)
        (`self.ReqApplyDamage` _asbp_mixamo_character 10.0 (`self.GetController`) self)))
    (set `local.OnceAttack` true)))

(fn `OnRep_IsClose`
  (`self.AttackMontage`)
  (`KismetSystemLibrary.PrintString` "on Rep is Close" true true (struct :`R` 1.0 :`G` 0.042313 :`A` 1.0)))

(fn `UserConstructionScript`)