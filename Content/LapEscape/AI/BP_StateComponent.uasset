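; BP_StateComponent is an AI state component that tracks a health value for its owner.
; SetHP subtracts damage, clamps the result between empty and full health, and returns whether health has reached zero.
; HP has a rep notify that prints a debug string and fires an UpdateHP event dispatcher so listeners can react to replicated changes.
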(fn `OnRep_HP`
  (`KismetSystemLibrary.PrintString` (`KismetStringLibrary.Concat_StrStr` "AI_state_onRepHP :  " (`KismetSystemLibrary.GetDisplayName` self)) true true (struct :`G` 0.66 :`B` 1.0 :`A` 1.0) 10.0)
  (`self.EventDispatcher_UpdateHP`))

(fn `SetHP`
  (params (Damage :type "Float (double-precision)"))
  (returns (IsDeath :type Boolean))
  (bind _output_get (set `self.HP` (`KismetMathLibrary.FClamp` (- (`self.HP`) Damage) 0.0 100.0)))
  (return (<= _output_get 0.0)))