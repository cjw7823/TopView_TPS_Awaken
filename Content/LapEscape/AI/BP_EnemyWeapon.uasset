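; BP_EnemyWeapon is an enemy projectile that damages the player character on contact.
; It takes its direction from the owning enemy's forward vector at BeginPlay, then moves a fixed step and rolls every tick, without delta-time scaling.
; Overlaps ignore AI enemies; anything else hides the mesh and disables its collision without destroying the actor.
; Hits on BP_MixamoCharacter route damage through the owner's ReqApplyDamage.
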(event `self.ReceiveBeginPlay`
  (set `self.MoveVector` (`self.GetActorForwardVector` (`self.OwnerEnemy`))))

(event `self.ReceiveTick`
  (params (DeltaSeconds :type "Float (single-precision)"))
  (bind _returnvalue_roll (`KismetMathLibrary.BreakRotator` (`self.K2_GetActorRotation`)))
  (`self.K2_SetActorLocationAndRotation` (+ (`self.K2_GetActorLocation`) (* (`self.MoveVector`) 10.0)) (`KismetMathLibrary.MakeRotator` (+ _returnvalue_roll 10.0))))

(event `self.StaticMesh.OnComponentBeginOverlap`
  (params (OverlappedComponent :type "PrimitiveComponent Object Reference") (OtherActor :type "Actor Object Reference") (OtherComp :type "PrimitiveComponent Object Reference") (OtherBodyIndex :type Integer) (bFromSweep :type Boolean) (SweepResult :type "HitResult Structure (by ref)"))
  (bind _staticmesh (`self.StaticMesh`))
  (bind _ownerenemy (`self.OwnerEnemy`))
  (cast `/Game/LapEscape/AI/BP_AI_Enemy` OtherActor
    (:`CastFailed`
      (`SceneComponent.SetVisibility` _staticmesh false false)
      (`PrimitiveComponent.SetCollisionEnabled` _staticmesh "NoCollision")
      (bind _asbp_mixamo_character (cast `/Game/LapEscape/GameMode/BP_MixamoCharacter` OtherActor))
      (`/Game/LapEscape/AI/BP_AI_Enemy.ReqApplyDamage` _ownerenemy _asbp_mixamo_character 10.0 (`Pawn.GetController` _ownerenemy) self (0.0 0.0 0.0) (0.0 0.0 0.0)))))

(fn `UserConstructionScript`)