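; Networked top-down player character for LapEscape with zoom, shooting, reloading, dodging and weapon pickup.
; Input flows through Req server and Res client events, driving weapons via BPI_Weapon and updating the HUD.
; Weapons fill main and pistol slots; damage outside dodges goes to PlayerState HP.
; Cursor-to-screen-center angle sets aim yaw; firing slows movement via OnRep and lerps the moving body toward aim, while the skill's response is empty.
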(event `InputAxis|Turn` :overrideparent false
  (params (AxisValue :type "Float (single-precision)"))
  ;[0 0 0] 마우스 회전(사용 안함)
)

(event `InputAxis|MoveForward` :overrideparent false
  (params (AxisValue :type "Float (single-precision)"))
  ;[1 1 1] W,S,A,D 이동
  (`self.AddMovementInput` (`KismetMathLibrary.GetForwardVector` (`KismetMathLibrary.MakeRotator` 0.0 0.0 (.yaw (`self.GetControlRotation`)))) AxisValue))

(event `InputAxis|LookUp` :overrideparent false
  (params (AxisValue :type "Float (single-precision)"))
  ;[0 0 0] 마우스 회전(사용 안함)
)

(event `InputAction|Jump` :overrideparent false
  (params (Key :type "Key Structure"))
  ;[0 0 0] Jump(사용 안함)
)

(event `InputAxis|MoveRight` :overrideparent false
  (params (AxisValue :type "Float (single-precision)"))
  ;[1 1 1] W,S,A,D 이동
  (`self.AddMovementInput` (`KismetMathLibrary.GetRightVector` (`KismetMathLibrary.MakeRotator` 0.0 0.0 (.yaw (`self.GetControlRotation`)))) AxisValue))

(event `InputAxisKey|MouseWheelAxis`
  (params (AxisValue :type "Float (single-precision)"))
  (bind _springarm (`self.SpringArm`))
  ;[1 1 1] 화면 확대/축소
  (bind _output_get (set `SpringArmComponent.TargetArmLength` (`KismetMathLibrary.FClamp` (+ (* AxisValue -100.0) (`SpringArmComponent.TargetArmLength` (`self.SpringArm`))) 300.0 800.0) _springarm))
  (set `SpringArmComponent.SocketOffset` (`KismetMathLibrary.MakeVector` 0.0 0.0 _output_get) _springarm))

(event `ReqReload`
  ;[1 0 0] (Server) Reload
  (`self.ResReload`))

(event `Key|R`
  (params (Key :type "Key Structure"))
  ;[1 1 1] Reload
  (:`Pressed`
    (`self.ReqReload`)))

(event `self.ReceiveAnyDamage`
  (params (Damage :type "Float (single-precision)") (DamageType :type "DamageType Object Reference") (InstigatedBy :type "Controller Object Reference") (DamageCauser :type "Actor Object Reference"))
  ;[1 0 0] (Server)AnyDamage 요청
  (if (`self.NotDodge`)
    (bind _asbp_my_player_state (cast `/Game/LapEscape/GameMode/BP_MyPlayerState` (`self.PlayerState`)))
    (`/Game/LapEscape/GameMode/BP_MyPlayerState.SetHP` _asbp_my_player_state Damage)
    (`KismetSystemLibrary.PrintString` (`KismetStringLibrary.Conv_DoubleToString` (`/Game/LapEscape/GameMode/BP_MyPlayerState.CurHP` _asbp_my_player_state)))))

(event `ResReload`
  (bind _attachedactor (`self.AttachedActor`))
  ;[1 1 1] (Client) Reload
  (`/Engine/EditorBlueprintResources/StandardMacros.IsValid` _attachedactor
    (:`Is Valid`
      (if (`KismetSystemLibrary.DoesImplementInterface` _attachedactor "/Game/LapEscape/Blueprints/Weapon/BPI_Weapon.BPI_Weapon_C")
        (message `/Game/LapEscape/Blueprints/Weapon/BPI_Weapon.Reload Montage` _attachedactor)))))

(event `ResPickUp`
  (params (PickupActor :type "Actor Object Reference"))
  ;[1 1 1] (Client)Pick Up
  (`self.Do Pickup` PickupActor)
  (if (== self (`GameplayStatics.GetPlayerCharacter` 0))
    (bind _asbp_my_hud (cast `/Game/LapEscape/GameMode/BP_MyHUD` (`PlayerController.GetHUD` (`GameplayStatics.GetPlayerController` 0))))
    (`/Game/LapEscape/Widget/MasterWidget/InGameMasterWidget.WeaponWidget Visible` (`/Game/LapEscape/GameMode/BP_MyHUD.InGameMasterWidget` _asbp_my_hud) (`self.AttachedActor`))))

(event `ReqShootPressed`
  ;[1 0 0] (Server) 요청
  (if (not (`self.IsDeath`))
    (`self.ResShootPressed`)))

(event `InputAction|PickUP`
  (params (Key :type "Key Structure"))
  ;[1 1 1] Pick Up
  (:`Pressed`
    (`self.ReqPickUp`)))

(event `self.ReceiveTick`
  (params (DeltaSeconds :type "Float (single-precision)"))
  (bind (_returnvalue_roll _returnvalue_pitch _returnvalue_yaw) (`KismetMathLibrary.BreakRotator` (`SceneComponent.K2_GetComponentRotation` (`self.Mesh`))))
  ;[1 1 1] Tick : Set RotationZ
  (if (== (`GameplayStatics.GetPlayerController` 0) (`self.GetOwner`))
    (`/Engine/EditorBlueprintResources/StandardMacros.IsValid` (`self.AttachedActor`)
      (:`Is Valid`
        (`self.ReqUpdateRotationZ` (- (`self.FindRotation`) _returnvalue_yaw))
        ;[1 1 1] Tick : Character Lerp Rotation
        (if (and (not (`KismetMathLibrary.NearlyEqual_FloatFloat` 0.0 (`KismetMathLibrary.VSize` (`self.GetVelocity`)) 1.0)) (`self.OnTriger`) (`self.NotDodge`))
          (`self.LerpRotation`))))))

(event `InputAction|Shoot`
  (params (Key :type "Key Structure"))
  ;[1 1 1] Shoot
  (:`Pressed`
    (`self.ReqShootPressed`))
  (:`Released`
    (`self.ReqShootReleased`)))

(event `ReqShootReleased`
  ;[1 0 0] (Server) 요청
  (if (not (`self.IsDeath`))
    (`self.ResShootReleased`)))

(event `ReqPickUp`
  ;[1 0 0] (Server)Pick Up
  (bind _nearestweapon (`self.FindNearWeapon`))
  (`/Engine/EditorBlueprintResources/StandardMacros.IsValid` _nearestweapon
    (:`Is Valid`
      (`self.SetOwner` _nearestweapon (`self.GetController`)))
    (:`Is Not Valid`
      _))
  (`self.ResPickUp` _nearestweapon))

(event `ResShootPressed`
  (bind _attachedactor (`self.AttachedActor`))
  ;[1 1 1] (Client) 수신
  (`/Engine/EditorBlueprintResources/StandardMacros.IsValid` _attachedactor
    (:`Is Valid`
      (if (`KismetSystemLibrary.DoesImplementInterface` _attachedactor "/Game/LapEscape/Blueprints/Weapon/BPI_Weapon.BPI_Weapon_C")
        (message `/Game/LapEscape/Blueprints/Weapon/BPI_Weapon.PullTriger` _attachedactor self)
        (set `self.OnTriger` true)))))

(event `ReqUpdateRotationZ`
  (params (RotationZ :type "Float (double-precision)"))
  ;[1 0 0] (Server) Set RotationZ
  (set `self.RotationZ` RotationZ))

(event `ReqDodge`
  ;[1 0 0] (Server)Dodge
  (if (`self.NotDodge`)
    (`self.ResDodge`)))

(event `Key|SpaceBar`
  (params (Key :type "Key Structure"))
  ;[1 1 1] Dodge
  (:`Pressed`
    (`self.ReqDodge`)))

(event `ResShootReleased`
  (bind _attachedactor (`self.AttachedActor`))
  ;[1 1 1] (Client) 수신
  (`/Engine/EditorBlueprintResources/StandardMacros.IsValid` _attachedactor
    (:`Is Valid`
      (if (`KismetSystemLibrary.DoesImplementInterface` _attachedactor "/Game/LapEscape/Blueprints/Weapon/BPI_Weapon.BPI_Weapon_C")
        (message `/Game/LapEscape/Blueprints/Weapon/BPI_Weapon.ReleaseTriger` _attachedactor self)
        (set `self.OnTriger` false)))))

(event `ResDodge`
  ;[1 1 1] (Client)Dodge
  (`self.K2_SetActorRotation` (`KismetMathLibrary.Conv_VectorToRotator` (`self.GetVelocity`)) true)
  (set `self.NotDodge` false)
  (`self.PlayAnimMontage` "/Game/Mannequin/MixamoAnim/Dodge_Montage.Dodge_Montage" 2.5))

(event `InputAction|Q Skill`
  (params (Key :type "Key Structure"))
  ;[1 1 1] Press Skill
  (:`Pressed`
    (`self.ReqSkill`)
    (`self.SkillCool`)))

(event `ReqSkill`
  ;[1 0 0] (Server) Skill
  (`self.ResSkill`))

(event `SkillCool`
  ;[1 1 1] Skill
  (bind _asbp_my_hud (cast `/Game/LapEscape/GameMode/BP_MyHUD` (`PlayerController.GetHUD` (`GameplayStatics.GetPlayerController` 0))))
  (bind _ingamemasterwidget (`/Game/LapEscape/GameMode/BP_MyHUD.InGameMasterWidget` _asbp_my_hud))
  (message `/Game/LapEscape/Blueprints/BPI_Skill.ActiveSkill` (`/Game/LapEscape/Widget/MasterWidget/InGameMasterWidget.SkillWidgetSteamPack` _ingamemasterwidget))
  (message `/Game/LapEscape/Blueprints/BPI_Skill.ActiveSkill` (`/Game/LapEscape/Widget/MasterWidget/InGameMasterWidget.SkillWidgetHeal` _ingamemasterwidget)))

(event `ResSkill`)

(fn `DiffWeapon`
  (params (PickupActor :type "Actor Object Reference"))
  (returns (DiffclassWeapon :type Boolean) (NotCurSlot :type "Actor Object Reference"))
  (cast `/Game/LapEscape/Blueprints/Weapon/BP_Pistol` PickupActor
    (:`then`
      (cast `/Game/LapEscape/Blueprints/Weapon/BP_Pistol` (`self.AttachedActor`)
        (:`then`
          (return false null))
        (:`CastFailed`
          (return true (`self.SubWeaponSlot`)))))
    (:`CastFailed`
      (cast `/Game/LapEscape/Blueprints/Weapon/BP_Pistol` (`self.AttachedActor`)
        (:`then`
          (return true (`self.MainWeaponSlot`)))
        (:`CastFailed`
          (return false null))))))

(fn `Do Pickup`
  (params (PickupActor :type "Actor Object Reference"))
  (bind (_diffclassweapon _notcurslot) (`self.DiffWeapon` PickupActor))
  (bind _attachedactor (`self.AttachedActor`))
  (`/Engine/EditorBlueprintResources/StandardMacros.IsValid` PickupActor
    (:`Is Valid`
      (`/Engine/EditorBlueprintResources/StandardMacros.IsValid` (`self.AttachedActor`)
        (:`Is Valid`
          (if _diffclassweapon
            (if (and (`KismetSystemLibrary.IsValid` (`self.MainWeaponSlot`)) (`KismetSystemLibrary.IsValid` (`self.SubWeaponSlot`)))
              (`SceneComponent.SetVisibility` (`Actor.RootComponent` _notcurslot) true false)
              (bind _result (message `/Game/LapEscape/Blueprints/Weapon/BPI_Weapon.Detach` _notcurslot self))
              (if _result
                (`SceneComponent.SetVisibility` (`Actor.RootComponent` (`self.AttachedActor`)) false false :!label _label)
                (bind _output_get (set `self.AttachedActor` PickupActor :!label _label_2))
                (bind _result_2 (message `/Game/LapEscape/Blueprints/Weapon/BPI_Weapon.Attach` _output_get self))
                (if _result_2
                  (cast `/Game/LapEscape/Blueprints/Weapon/BP_Pistol` _attachedactor
                    (:`then`
                      (bind _output_get_2 (set `self.SubWeaponSlot` _attachedactor))
                      (`KismetSystemLibrary.PrintString` (`KismetSystemLibrary.GetDisplayName` _output_get_2)))
                    (:`CastFailed`
                      (bind _output_get_3 (set `self.MainWeaponSlot` _attachedactor))
                      (`KismetSystemLibrary.PrintString` (`KismetSystemLibrary.GetDisplayName` _output_get_3))))
                  (else
                    (set `self.AttachedActor` null)
                    (`KismetSystemLibrary.PrintString` "Attach 실패"))))
              (else
                (goto _label)))
            (else
              (bind _result_3 (message `/Game/LapEscape/Blueprints/Weapon/BPI_Weapon.Detach` (`self.AttachedActor`) self))
              (if _result_3
                (goto _label_2)))))
        (:`Is Not Valid`
          (goto _label_2))))
    (:`Is Not Valid`
      (`/Engine/EditorBlueprintResources/StandardMacros.IsValid` (`self.AttachedActor`)
        (:`Is Valid`
          ;[1 1 1] Swap Weapon
          (`self.PlayAnimMontage` "/Game/Mannequin/MixamoAnim/Swap_Gun_Anim_Montage.Swap_Gun_Anim_Montage" 2.0))
        (:`Is Not Valid`
          (`KismetSystemLibrary.PrintString` "아무것도 안함."))))))

(fn `FindNearWeapon`
  (returns (NearestWeapon :type "Actor Object Reference"))
  (locals (NearestWP :type "Actor Object Reference") (NearestDist :type "Float (double-precision)" :default 10000.0))
  (for _array_element (`self.GetOverlappingActors` "/Script/Engine.Actor")
    (`/Engine/EditorBlueprintResources/StandardMacros.IsValid` (`self.GetOwner` _array_element)
      (:`Is Not Valid`
        (if (!= _array_element (`self.AttachedActor`))
          (if (`KismetSystemLibrary.DoesImplementInterface` _array_element "/Game/LapEscape/Blueprints/Weapon/BPI_Weapon.BPI_Weapon_C")
            (bind _returnvalue (`KismetMathLibrary.VSize` (- (`self.K2_GetActorLocation` _array_element) (`self.K2_GetActorLocation`))))
            (if (< _returnvalue (`local.NearestDist`))
              (set `local.NearestDist` _returnvalue)
              (set `local.NearestWP` _array_element)))))))
  (return (`local.NearestWP`)))

(fn `FindRotation`
  (returns (ReturnValue :type "Float (double-precision)"))
  (bind (_returnvalue_x _returnvalue_y) (`KismetMathLibrary.BreakVector2D` (`WidgetLayoutLibrary.GetViewportSize`)))
  (bind (_locationx _locationy) (`PlayerController.GetMousePosition` (`GameplayStatics.GetPlayerController` 0)))
  (bind (_returnvalue_roll _returnvalue_pitch _returnvalue_yaw) (`KismetMathLibrary.BreakRotator` (`KismetMathLibrary.FindLookAtRotation` (`KismetMathLibrary.MakeVector` (/ _returnvalue_x 2.0) (+ (/ _returnvalue_y 2.0) -50.0)) (`KismetMathLibrary.MakeVector` _locationx _locationy))))
  (return _returnvalue_yaw))

(fn `IsDeath`
  (returns (Death :type Boolean))
  (bind _asbp_my_player_state (cast `/Game/LapEscape/GameMode/BP_MyPlayerState` (`self.PlayerState`)))
  (return (<= (`/Game/LapEscape/GameMode/BP_MyPlayerState.CurHP` _asbp_my_player_state) 0.0)))

(fn `LerpRotation`
  (bind (_returnvalue_roll _returnvalue_pitch) (`KismetMathLibrary.BreakRotator` (`self.K2_GetActorRotation`)))
  (`self.K2_SetActorRotation` (`KismetMathLibrary.RLerp` (`self.K2_GetActorRotation`) (`KismetMathLibrary.MakeRotator` _returnvalue_roll _returnvalue_pitch (+ (`self.FindRotation`) 90.0)) 0.03 true)))

(fn `OnRep_OnTriger`
  (bind _charactermovement (`self.CharacterMovement`))
  (bind _charactermovement_2 (`self.CharacterMovement`))
  (if (`self.OnTriger`)
    (bind _asbp_my_player_state (cast `/Game/LapEscape/GameMode/BP_MyPlayerState` (`self.PlayerState`)))
    (set `CharacterMovementComponent.MaxWalkSpeed` (/ (* (`/Game/LapEscape/GameMode/BP_MyPlayerState.MaxWalkSpeed(custom)` _asbp_my_player_state) 2.0) 3.0) _charactermovement_2)
    (set `CharacterMovementComponent.RotationRate` (struct) _charactermovement_2)
    (else
      (bind _asbp_my_player_state_2 (cast `/Game/LapEscape/GameMode/BP_MyPlayerState` (`self.PlayerState`)))
      (set `CharacterMovementComponent.MaxWalkSpeed` (`/Game/LapEscape/GameMode/BP_MyPlayerState.MaxWalkSpeed(custom)` _asbp_my_player_state_2) _charactermovement)
      (set `CharacterMovementComponent.RotationRate` (struct :`Yaw` 360.0) _charactermovement))))

(fn `SwapWeapon`
  ;[1 1 1] 지금 무기가
  (cast `/Game/LapEscape/Blueprints/Weapon/BP_Pistol` (`self.AttachedActor`)
    (:`then`
      ;[1 1 1] 서브면 메인슬롯 확인
      (`/Engine/EditorBlueprintResources/StandardMacros.IsValid` (`self.MainWeaponSlot`)
        (:`Is Valid`
          (`SceneComponent.SetVisibility` (`Actor.RootComponent` (`self.SubWeaponSlot`)) false false)
          (`SceneComponent.SetVisibility` (`Actor.RootComponent` (`self.MainWeaponSlot`)) true false)
          (bind _output_get (set `self.AttachedActor` (`self.MainWeaponSlot`)))
          (bind _asbp_weapon (cast `/Game/LapEscape/Blueprints/Weapon/BP_Weapon` _output_get))
          (set `self.Type_Weapon` (`.Type_25_7807464E4B1535A814F454809CF8F6F8` (break `/Game/LapEscape/Data/ST_Weapon` (`/Game/LapEscape/Blueprints/Weapon/BP_Weapon.Weapon Data` _asbp_weapon))))
          (`KismetSystemLibrary.PrintString` "스왑 성공")
          (if (== self (`GameplayStatics.GetPlayerCharacter` 0)) :!label _label
            (bind _asbp_my_hud (cast `/Game/LapEscape/GameMode/BP_MyHUD` (`PlayerController.GetHUD` (`GameplayStatics.GetPlayerController` 0))))
            (`/Game/LapEscape/Widget/MasterWidget/InGameMasterWidget.WeaponWidget Visible` (`/Game/LapEscape/GameMode/BP_MyHUD.InGameMasterWidget` _asbp_my_hud) (`self.AttachedActor`))))
        (:`Is Not Valid`
          (`KismetSystemLibrary.PrintString` "스왑할 메인 무기가 없습니다."))))
    (:`CastFailed`
      ;[1 1 1] 메인이면 서브슬롯 확인
      (`/Engine/EditorBlueprintResources/StandardMacros.IsValid` (`self.SubWeaponSlot`)
        (:`Is Valid`
          (`SceneComponent.SetVisibility` (`Actor.RootComponent` (`self.SubWeaponSlot`)) true false)
          (`SceneComponent.SetVisibility` (`Actor.RootComponent` (`self.MainWeaponSlot`)) false false)
          (bind _output_get_2 (set `self.AttachedActor` (`self.SubWeaponSlot`)))
          (bind _asbp_weapon_2 (cast `/Game/LapEscape/Blueprints/Weapon/BP_Weapon` _output_get_2))
          (set `self.Type_Weapon` (`.Type_25_7807464E4B1535A814F454809CF8F6F8` (break `/Game/LapEscape/Data/ST_Weapon` (`/Game/LapEscape/Blueprints/Weapon/BP_Weapon.Weapon Data` _asbp_weapon_2))))
          (`KismetSystemLibrary.PrintString` "스왑 성공")
          (goto _label))
        (:`Is Not Valid`
          (`KismetSystemLibrary.PrintString` "스왑할 서브 무기가 없습니다."))))))

(fn `UserConstructionScript`)