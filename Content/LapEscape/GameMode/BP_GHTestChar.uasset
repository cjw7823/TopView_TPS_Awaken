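; BP_GHTestChar is a networked player character with WASD movement, wheel-zoomed camera, mouse-cursor aiming and a Q key for HUD skill widgets.
; Pickup and shooting use Req/Res server-to-client events, attaching, swapping, dropping or triggering the nearest unowned weapon through BPI_Weapon.
; Tick requests RotationZ updates from the cursor's screen-space angle while armed.
; OnRep_OnTriger freezes movement rotation during fire, while LerpRotation turns the body toward the cursor until nearly aligned.
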(event `InputAxis|Turn` :overrideparent false
  (params (AxisValue :type "Float (single-precision)"))
  ;[0 0 0] 마우스 회전(사용 안함)
)

(event `InputAxis|MoveForward` :overrideparent false
  (params (AxisValue :type "Float (single-precision)"))
  ;[1 1 1] W,S,A,D 이동
  (`self.AddMovementInput` (`KismetMathLibrary.GetForwardVector` (`KismetMathLibrary.MakeRotator` 0.0 0.0 (.yaw (`self.GetControlRotation`)))) AxisValue))

(event `InputAxis|LookUp` :overrideparent false
  (params (AxisValue :type "Float (single-precision)"))
  ;[0 0 0] 마우스 회전(사용 안함)
)

(event `InputAction|Jump` :overrideparent false
  (params (Key :type "Key Structure"))
  ;[0 0 0] Jump(사용 안함)
)

(event `InputAxis|MoveRight` :overrideparent false
  (params (AxisValue :type "Float (single-precision)"))
  ;[1 1 1] W,S,A,D 이동
  (`self.AddMovementInput` (`KismetMathLibrary.GetRightVector` (`KismetMathLibrary.MakeRotator` 0.0 0.0 (.yaw (`self.GetControlRotation`)))) AxisValue))

(event `InputAxisKey|MouseWheelAxis`
  (params (AxisValue :type "Float (single-precision)"))
  (bind _springarm (`self.SpringArm`))
  ;[1 1 1] 화면 확대/축소
  (bind _output_get (set `SpringArmComponent.TargetArmLength` (`KismetMathLibrary.FClamp` (+ (* AxisValue -100.0) (`SpringArmComponent.TargetArmLength` (`self.SpringArm`))) 300.0 1000.0) _springarm))
  (set `SpringArmComponent.SocketOffset` (`KismetMathLibrary.MakeVector` 0.0 0.0 _output_get) _springarm))

(event `Key|Q`
  (params (Key :type "Key Structure"))
  (:`Pressed`
    (bind _asbp_my_hud (cast `/Game/LapEscape/GameMode/BP_MyHUD` (`PlayerController.GetHUD` (`GameplayStatics.GetPlayerController` 0))))
    (bind _ingamemasterwidget (`/Game/LapEscape/GameMode/BP_MyHUD.InGameMasterWidget` _asbp_my_hud))
    (message `/Game/LapEscape/Blueprints/BPI_Skill.ActiveSkill` (`/Game/LapEscape/Widget/MasterWidget/InGameMasterWidget.SkillWidgetSteamPack` _ingamemasterwidget))
    (message `/Game/LapEscape/Blueprints/BPI_Skill.ActiveSkill` (`/Game/LapEscape/Widget/MasterWidget/InGameMasterWidget.SkillWidgetHeal` _ingamemasterwidget))))

(event `ResPickUp`
  (params (PickupActor :type "Actor Object Reference"))
  ;[1 1 1] (Client)Pick Up
  (`self.Do Pickup` PickupActor))

(event `ReqShootPressed`
  ;[1 0 0] (Server) 요청
  (if (not (`self.IsDeath`))
    (`self.ResShootPressed`)))

(event `InputAction|PickUP`
  (params (Key :type "Key Structure"))
  ;[1 1 1] Pick Up
  (:`Pressed`
    (`self.ReqPickUp`)))

(event `InputAction|Shoot`
  (params (Key :type "Key Structure"))
  ;[1 1 1] Shoot
  (:`Pressed`
    (`self.ReqShootPressed`))
  (:`Released`
    (`self.ReqShootReleased`)))

(event `ReqShootReleased`
  ;[1 0 0] (Server) 요청
  (if (not (`self.IsDeath`))
    (`self.ResShootReleased`)))

(event `ReqPickUp`
  ;[1 0 0] (Server)Pick Up
  (bind _nearestweapon (`self.FindNearWeapon`))
  (`/Engine/EditorBlueprintResources/StandardMacros.IsValid` _nearestweapon
    (:`Is Valid`
      (`self.SetOwner` _nearestweapon (`self.GetController`)))
    (:`Is Not Valid`
      _))
  (`self.ResPickUp` _nearestweapon))

(event `ResShootPressed`
  (bind _attachedactor (`self.AttachedActor`))
  ;[1 1 1] (Client) 수신
  (`/Engine/EditorBlueprintResources/StandardMacros.IsValid` _attachedactor
    (:`Is Valid`
      (if (`KismetSystemLibrary.DoesImplementInterface` _attachedactor "/Game/LapEscape/Blueprints/BPI_Weapon.BPI_Weapon_C")
        (message `/Game/LapEscape/Blueprints/BPI_Weapon.PullTriger` _attachedactor self)
        (set `self.OnTriger` true)))))

(event `self.ReceiveTick`
  (params (DeltaSeconds :type "Float (single-precision)"))
  ;[1 1 1] Tick : Set RotationZ
  (if (== (`GameplayStatics.GetPlayerController` 0) (`self.GetOwner`))
    (`/Engine/EditorBlueprintResources/StandardMacros.IsValid` (`self.AttachedActor`)
      (:`Is Valid`
        (`self.ReqUpdateRotationZ`)
        ;[1 1 1] Tick : Character Lerp Rotation
        (if (and (`self.OnTriger`) (`self.StopLerpRotation`))
          (`self.LerpRotation`))))))

(event `ResShootReleased`
  (bind _attachedactor (`self.AttachedActor`))
  ;[1 1 1] (Client) 수신
  (`/Engine/EditorBlueprintResources/StandardMacros.IsValid` _attachedactor
    (:`Is Valid`
      (if (`KismetSystemLibrary.DoesImplementInterface` _attachedactor "/Game/LapEscape/Blueprints/BPI_Weapon.BPI_Weapon_C")
        (message `/Game/LapEscape/Blueprints/BPI_Weapon.ReleaseTriger` _attachedactor self)
        (set `self.OnTriger` false)))))

(event `ReqUpdateRotationZ`
  (bind (_returnvalue_roll _returnvalue_pitch _returnvalue_yaw) (`KismetMathLibrary.BreakRotator` (`SceneComponent.K2_GetComponentRotation` (`self.Mesh`))))
  ;[1 0 0] (Server) Set RotationZ
  (set `self.RotationZ` (- (`self.FindRotation`) _returnvalue_yaw)))

(fn `Do Pickup`
  (params (PickupActor :type "Actor Object Reference"))
  (bind _attachedactor (`self.AttachedActor`))
  (bind _attachedactor_2 (`self.AttachedActor`))
  (`/Engine/EditorBlueprintResources/StandardMacros.IsValid` PickupActor
    (:`Is Valid`
      (`/Engine/EditorBlueprintResources/StandardMacros.IsValid` _attachedactor
        (:`Is Valid`
          (bind _result (message `/Game/LapEscape/Blueprints/BPI_Weapon.Detach` _attachedactor self))
          (if _result
            (bind _output_get (set `self.AttachedActor` PickupActor :!label _label))
            (bind _result_2 (message `/Game/LapEscape/Blueprints/BPI_Weapon.Attach` _output_get self))
            (if (not _result_2)
              (set `self.AttachedActor` null))))
        (:`Is Not Valid`
          (goto _label))))
    (:`Is Not Valid`
      ;[1 1 1] 잡을 수 있는 무기가 없고 이미 무기를 가지고 있다면 버린다.
      (`/Engine/EditorBlueprintResources/StandardMacros.IsValid` _attachedactor_2
        (:`Is Valid`
          (bind _result_3 (message `/Game/LapEscape/Blueprints/BPI_Weapon.Detach` _attachedactor_2 self))
          (if _result_3
            (set `self.AttachedActor` null)))))))

(fn `FindNearWeapon`
  (returns (NearestWeapon :type "Actor Object Reference"))
  (locals (NearestWP :type "Actor Object Reference") (NearestDist :type "Float (double-precision)" :default 10000.0))
  (for _array_element (`self.GetOverlappingActors` "/Script/Engine.Actor")
    (`/Engine/EditorBlueprintResources/StandardMacros.IsValid` (`self.GetOwner` _array_element)
      (:`Is Not Valid`
        (if (!= _array_element (`self.AttachedActor`))
          (if (`KismetSystemLibrary.DoesImplementInterface` _array_element "/Game/LapEscape/Blueprints/BPI_Weapon.BPI_Weapon_C")
            (bind _returnvalue (`KismetMathLibrary.VSize` (- (`self.K2_GetActorLocation` _array_element) (`self.K2_GetActorLocation`))))
            (if (< _returnvalue (`local.NearestDist`))
              (set `local.NearestDist` _returnvalue)
              (set `local.NearestWP` _array_element)))))))
  (return (`local.NearestWP`)))

(fn `FindRotation`
  (returns (ReturnValue :type "Float (double-precision)"))
  (bind (_returnvalue_x _returnvalue_y) (`KismetMathLibrary.BreakVector2D` (`WidgetLayoutLibrary.GetViewportSize`)))
  (bind (_locationx _locationy) (`PlayerController.GetMousePosition` (`GameplayStatics.GetPlayerController` 0)))
  (bind (_returnvalue_roll _returnvalue_pitch _returnvalue_yaw) (`KismetMathLibrary.BreakRotator` (`KismetMathLibrary.FindLookAtRotation` (`KismetMathLibrary.MakeVector` (/ _returnvalue_x 2.0) (+ (/ _returnvalue_y 2.0) -50.0)) (`KismetMathLibrary.MakeVector` _locationx _locationy))))
  (return _returnvalue_yaw))

(fn `IsDeath`
  (returns (Death :type Boolean))
  (bind _asbp_my_player_state (cast `/Game/LapEscape/GameMode/BP_MyPlayerState` (`self.PlayerState`)))
  (return (<= (`/Game/LapEscape/GameMode/BP_MyPlayerState.HP` _asbp_my_player_state) 0.0)))

(fn `LerpRotation`
  (bind (_returnvalue_roll _returnvalue_pitch) (`KismetMathLibrary.BreakRotator` (`self.K2_GetActorRotation`)))
  (bind (_returnvalue_roll_2 _returnvalue_pitch_2 _returnvalue_yaw) (`KismetMathLibrary.BreakRotator` (`self.K2_GetActorRotation`)))
  (`self.K2_SetActorRotation` (`KismetMathLibrary.RLerp` (`self.K2_GetActorRotation`) (`KismetMathLibrary.MakeRotator` _returnvalue_roll _returnvalue_pitch (+ (`self.FindRotation`) 90.0)) 0.05 true))
  (if (`KismetMathLibrary.NearlyEqual_FloatFloat` _returnvalue_yaw (+ (`self.FindRotation`) 90.0) 8.0)
    (set `self.StopLerpRotation` false)))

(fn `OnRep_OnTriger`
  (if (`self.OnTriger`)
    (set `CharacterMovementComponent.RotationRate` (struct) (`self.CharacterMovement`))
    (else
      (set `CharacterMovementComponent.RotationRate` (struct :`Yaw` 360.0) (`self.CharacterMovement`))
      (set `self.StopLerpRotation` true))))

(fn `UserConstructionScript`)