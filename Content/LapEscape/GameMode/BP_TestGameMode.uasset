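; BP_TestGameMode is a LapEscape game mode Blueprint that hands out random, non-repeating player starts.
; On BeginPlay it caches every PlayerStart actor in the level into the PlayerStarts array.
; SetPlayerStart picks a random entry, removes it from the array and returns it, with no refill or empty-array check.
; Nothing in this Blueprint calls SetPlayerStart.
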(event `self.ReceiveBeginPlay`
  (bind _outactors (`GameplayStatics.GetAllActorsOfClass` "/Script/Engine.PlayerStart"))
  (set `self.Player Starts` _outactors))

(fn `SetPlayerStart`
  (returns (PlayerStart :type "Actor Object Reference"))
  (bind _player_starts (`self.Player Starts`))
  (bind _output_get (set `self.Selected Player Start` (`|GetArrayItem` _player_starts (`KismetMathLibrary.RandomInteger` (`KismetArrayLibrary.Array_Length` _player_starts)))))
  (`KismetArrayLibrary.Array_RemoveItem` _player_starts _output_get)
  (return (`self.Selected Player Start`)))

(fn `UserConstructionScript`)