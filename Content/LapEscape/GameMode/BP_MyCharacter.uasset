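; BP_MyCharacter is the LapEscape player character, handling movement, camera zoom and weapon pickup.
; Movement follows control yaw and mouse turns only horizontally, with pitch and jump left unwired.
; Mouse wheel changes clamped spring arm length and matches socket height to it, raising the camera when zooming out.
; PickUP detaches any held actor, then attaches the nearest overlapping BPI_Weapon actor through attach/detach messages.
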(event `InputAxis|Turn` :overrideparent false
  (params (AxisValue :type "Float (single-precision)"))
  ;[1 1 1] 마우스 회전
  (`self.AddControllerYawInput` AxisValue))

(event `InputAxis|MoveForward` :overrideparent false
  (params (AxisValue :type "Float (single-precision)"))
  ;[1 1 1] W,S,A,D 이동
  (`self.AddMovementInput` (`KismetMathLibrary.GetForwardVector` (`KismetMathLibrary.MakeRotator` 0.0 0.0 (.yaw (`self.GetControlRotation`)))) AxisValue))

(event `InputAxis|LookUp` :overrideparent false
  (params (AxisValue :type "Float (single-precision)"))
  ;[1 1 1] 마우스 회전
)

(event `InputAction|Jump` :overrideparent false
  (params (Key :type "Key Structure"))
  ;[0 0 0] Jump(사용 안함)
)

(event `InputAxis|MoveRight` :overrideparent false
  (params (AxisValue :type "Float (single-precision)"))
  ;[1 1 1] W,S,A,D 이동
  (`self.AddMovementInput` (`KismetMathLibrary.GetRightVector` (`KismetMathLibrary.MakeRotator` 0.0 0.0 (.yaw (`self.GetControlRotation`)))) AxisValue))

(event `InputAxisKey|MouseWheelAxis`
  (params (AxisValue :type "Float (single-precision)"))
  (bind _springarm (`self.SpringArm`))
  ;[1 1 1] 화면 확대/축소
  (bind _output_get (set `SpringArmComponent.TargetArmLength` (`KismetMathLibrary.FClamp` (+ (* AxisValue -100.0) (`SpringArmComponent.TargetArmLength` (`self.SpringArm`))) 300.0 1000.0) _springarm))
  (set `SpringArmComponent.SocketOffset` (`KismetMathLibrary.MakeVector` 0.0 0.0 _output_get) _springarm))

(event `InputAction|PickUP`
  (params (Key :type "Key Structure"))
  (:`Pressed`
    (`self.ReqPickUp`)))

(event `ReqPickUp`
  (`self.DoPickup`))

(fn `DoPickup`
  (bind _attachedactor (`self.AttachedActor`))
  (`/Engine/EditorBlueprintResources/StandardMacros.IsValid` _attachedactor
    (:`Is Valid`
      (message `/Game/LapEscape/Blueprints/BPI_Weapon.Detach` _attachedactor null))
    (:`Is Not Valid`
      _))
  (bind _nearestweapon (`self.FindNearWeapon`))
  (bind _output_get (set `self.AttachedActor` _nearestweapon))
  (message `/Game/LapEscape/Blueprints/BPI_Weapon.Attach` _output_get self))

(fn `FindNearWeapon`
  (returns (NearestWeapon :type "Actor Object Reference"))
  (locals (NearestWP :type "Actor Object Reference") (NearestDist :type "Float (double-precision)" :default 10000.0))
  (for _array_element (`self.GetOverlappingActors` "/Script/Engine.Actor")
    (if (`KismetSystemLibrary.DoesImplementInterface` _array_element "/Game/LapEscape/Blueprints/BPI_Weapon.BPI_Weapon_C")
      (bind _returnvalue (`KismetMathLibrary.VSize` (- (`self.K2_GetActorLocation` _array_element) (`self.K2_GetActorLocation`))))
      (if (< _returnvalue (`local.NearestDist`))
        (set `local.NearestDist` _returnvalue)
        (set `local.NearestWP` _array_element))))
  (return (`local.NearestWP`)))

(fn `UserConstructionScript`)