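; Player state for LapEscape that holds health, walk speed, heal rate and skill tick stats, and handles gold-bought upgrades to them.
; BeginPlay loads the stats from Awaken_GameInstance and starts at full HP.
; Upgrade requests require more gold than the cost, deduct it from BP_MyGameState, and write gold and stat back to the game instance.
; Damage and clamped healing change CurHP, whose OnRep fires an HP update dispatcher.
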(event `self.ReceiveBeginPlay`
  (bind _asawaken_game_instance (cast `/Game/LapEscape/Awaken_GameInstance` (`GameplayStatics.GetGameInstance`)))
  (bind _output_get (set `self.MaxHP` (`/Game/LapEscape/Awaken_GameInstance.MaxHP` _asawaken_game_instance)))
  (set `self.CurHP` _output_get)
  (set `self.MaxWalkSpeed(custom)` (`/Game/LapEscape/Awaken_GameInstance.MaxWalkSpeed(custom)` _asawaken_game_instance))
  (set `self.Healrate` (`/Game/LapEscape/Awaken_GameInstance.Healrate` _asawaken_game_instance))
  (set `self.MaxSkillTick` (`/Game/LapEscape/Awaken_GameInstance.MaxSkillTick` _asawaken_game_instance)))

(event `ReqMaxHPup`
  (bind _asbp_my_game_state (cast `/Game/LapEscape/GameMode/BP_MyGameState` (`GameplayStatics.GetGameState`)))
  (bind _returnvalue (- (`/Game/LapEscape/GameMode/BP_MyGameState.Gold` _asbp_my_game_state) 5))
  (if (> _returnvalue 0)
    (bind _output_get (set `/Game/LapEscape/GameMode/BP_MyGameState.Gold` _returnvalue _asbp_my_game_state))
    (bind _asawaken_game_instance (cast `/Game/LapEscape/Awaken_GameInstance` (`GameplayStatics.GetGameInstance`)))
    (set `/Game/LapEscape/Awaken_GameInstance.Gold` _output_get _asawaken_game_instance)
    (bind _output_get_2 (set `self.MaxHP` (+ (`self.MaxHP`) 10.0)))
    (set `self.CurHP` (+ (`self.CurHP`) 10.0))
    (bind _asawaken_game_instance_2 (cast `/Game/LapEscape/Awaken_GameInstance` (`GameplayStatics.GetGameInstance`)))
    (set `/Game/LapEscape/Awaken_GameInstance.MaxHP` _output_get_2 _asawaken_game_instance_2)))

(event `ReqEatHealActor`
  (`self.HealHP` (`self.Healrate`)))

(event `ReqHealrateup`
  (bind _asbp_my_game_state (cast `/Game/LapEscape/GameMode/BP_MyGameState` (`GameplayStatics.GetGameState`)))
  (bind _returnvalue (- (`/Game/LapEscape/GameMode/BP_MyGameState.Gold` _asbp_my_game_state) 2))
  (if (> _returnvalue 0)
    (bind _output_get (set `/Game/LapEscape/GameMode/BP_MyGameState.Gold` _returnvalue _asbp_my_game_state))
    (bind _asawaken_game_instance (cast `/Game/LapEscape/Awaken_GameInstance` (`GameplayStatics.GetGameInstance`)))
    (set `/Game/LapEscape/Awaken_GameInstance.Gold` _output_get _asawaken_game_instance)
    (bind _output_get_2 (set `self.Healrate` (+ (`self.Healrate`) 10.0)))
    (bind _asawaken_game_instance_2 (cast `/Game/LapEscape/Awaken_GameInstance` (`GameplayStatics.GetGameInstance`)))
    (set `/Game/LapEscape/Awaken_GameInstance.Healrate` _output_get_2 _asawaken_game_instance_2)))

(event `ReqMaxSpeedup`
  (bind _asbp_my_game_state (cast `/Game/LapEscape/GameMode/BP_MyGameState` (`GameplayStatics.GetGameState`)))
  (bind _returnvalue (- (`/Game/LapEscape/GameMode/BP_MyGameState.Gold` _asbp_my_game_state) 5))
  (if (> _returnvalue 0)
    (bind _output_get (set `/Game/LapEscape/GameMode/BP_MyGameState.Gold` _returnvalue _asbp_my_game_state))
    (bind _asawaken_game_instance (cast `/Game/LapEscape/Awaken_GameInstance` (`GameplayStatics.GetGameInstance`)))
    (set `/Game/LapEscape/Awaken_GameInstance.Gold` _output_get _asawaken_game_instance)
    (bind _output_get_2 (set `self.MaxWalkSpeed(custom)` (+ (`self.MaxWalkSpeed(custom)`) 50.0)))
    (bind _asawaken_game_instance_2 (cast `/Game/LapEscape/Awaken_GameInstance` (`GameplayStatics.GetGameInstance`)))
    (set `/Game/LapEscape/Awaken_GameInstance.MaxWalkSpeed(custom)` _output_get_2 _asawaken_game_instance_2)))

(event `ReqMaxSkillTickup`
  (bind _asbp_my_game_state (cast `/Game/LapEscape/GameMode/BP_MyGameState` (`GameplayStatics.GetGameState`)))
  (bind _returnvalue (- (`/Game/LapEscape/GameMode/BP_MyGameState.Gold` _asbp_my_game_state) 5))
  (if (> _returnvalue 0)
    (bind _output_get (set `/Game/LapEscape/GameMode/BP_MyGameState.Gold` _returnvalue _asbp_my_game_state))
    (bind _asawaken_game_instance (cast `/Game/LapEscape/Awaken_GameInstance` (`GameplayStatics.GetGameInstance`)))
    (set `/Game/LapEscape/Awaken_GameInstance.Gold` _output_get _asawaken_game_instance)
    (bind _result (`/Engine/EditorBlueprintResources/StandardMacros.IncrementInt` (`self.MaxSkillTick`))
      (:`  `
        (`KismetSystemLibrary.PrintString` (`KismetStringLibrary.Conv_IntToString` _result) false false)
        (bind _asawaken_game_instance_2 (cast `/Game/LapEscape/Awaken_GameInstance` (`GameplayStatics.GetGameInstance`)))
        (set `/Game/LapEscape/Awaken_GameInstance.MaxSkillTick` _result _asawaken_game_instance_2)))))

(fn `HealHP`
  (params (Heal :type "Float (double-precision)"))
  (bind _output_get (set `self.CurHP` (+ (`self.CurHP`) Heal)))
  (if (not (<= _output_get (`self.MaxHP`)))
    (set `self.CurHP` (`self.MaxHP`))))

(fn `OnRep_CurHP`
  (`self.EventDispatcher_Update_HP`))

(fn `SetHP`
  (params (Damage :type "Float (double-precision)"))
  (set `self.CurHP` (- (`self.CurHP`) Damage)))

(fn `UserConstructionScript`)