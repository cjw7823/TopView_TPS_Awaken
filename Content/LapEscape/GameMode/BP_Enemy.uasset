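; BP_Enemy is an enemy Blueprint in LapEscape that can pick up and swap weapons.
; FindNearWeapon scans overlapping actors for those implementing BPI_Weapon and returns the nearest by distance.
; DoPickup detaches any held actor through DetachMessage, stores the search result as AttachedActor, and sends it AttachMessage with itself, without a validity check.
; The file shows no event or caller that triggers the pickup.
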(fn `DoPickup`
  (bind _attachedactor (`self.AttachedActor`))
  (`/Engine/EditorBlueprintResources/StandardMacros.IsValid` _attachedactor
    (:`Is Valid`
      (message `/Game/LapEscape/Blueprints/BPI_Weapon.Detach` _attachedactor null))
    (:`Is Not Valid`
      _))
  (bind _nearestweapon (`self.FindNearWeapon`))
  (bind _output_get (set `self.AttachedActor` _nearestweapon))
  (message `/Game/LapEscape/Blueprints/BPI_Weapon.Attach` _output_get self))

(fn `FindNearWeapon`
  (returns (NearestWeapon :type "Actor Object Reference"))
  (locals (NearestWP :type "Actor Object Reference") (NearestDist :type "Float (double-precision)" :default 10000.0))
  (for _array_element (`self.GetOverlappingActors` "/Script/Engine.Actor")
    (if (`KismetSystemLibrary.DoesImplementInterface` _array_element "/Game/LapEscape/Blueprints/BPI_Weapon.BPI_Weapon_C")
      (bind _returnvalue (`KismetMathLibrary.VSize` (- (`self.K2_GetActorLocation` _array_element) (`self.K2_GetActorLocation`))))
      (if (< _returnvalue (`local.NearestDist`))
        (set `local.NearestDist` _returnvalue)
        (set `local.NearestWP` _array_element))))
  (return (`local.NearestWP`)))

(fn `UserConstructionScript`)