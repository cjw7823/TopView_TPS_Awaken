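; Player controller that spawns the player's chosen character, restores its weapon loadout and handles text chat.
; On BeginPlay, the local controller creates the chat widget and sends Game Instance selections to the server, which spawns and possesses the pawn at a GameMode-chosen start.
; Outside RepairShop1, it attaches a pistol and a rifle or shotgun with saved upgrade stats.
; Chat messages relay through every controller, and possession fires a rotate dispatcher.
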(event `self.ReceiveBeginPlay`
  ;[1 1 1] BeginPlay
  (`self.Get_ChooseCharacter_inGameinstance`))

(event `Get_ChooseCharacter_inGameinstance`
  ;[1 1 1] (Client) Game Instance에서 선택한 캐릭 정보 가져오기.
  (if (== self (`GameplayStatics.GetPlayerController` 0))
    (bind _asawaken_game_instance (cast `/Game/LapEscape/Awaken_GameInstance` (`GameplayStatics.GetGameInstance`)))
    (`self.ReqSpawnCharacter` (`/Game/LapEscape/Awaken_GameInstance.ChooseCharacter` _asawaken_game_instance) (`/Game/LapEscape/Awaken_GameInstance.MainWeaponSlotClass` _asawaken_game_instance) (`/Game/LapEscape/Awaken_GameInstance.Upgrade Damage` _asawaken_game_instance) (`/Game/LapEscape/Awaken_GameInstance.ShootingSpeed` _asawaken_game_instance) (`/Game/LapEscape/Awaken_GameInstance.ReloadSpeed` _asawaken_game_instance) (`/Game/LapEscape/Awaken_GameInstance.MaxAmmo` _asawaken_game_instance))
    ;[1 1 1] 채팅 위젯 생성
    (bind _returnvalue (`|CreateWidget` "/Game/LapEscape/Widget/ChatWidget/ChattingWidget.ChattingWidget_C"))
    (bind _output_get (set `self.ChattingWidget` _returnvalue))
    (`UserWidget.AddToViewport` _output_get 0)
    (bind _asawaken_game_instance_2 (cast `/Game/LapEscape/Awaken_GameInstance` (`GameplayStatics.GetGameInstance`)))
    (set `self.NickName` (`/Game/LapEscape/Awaken_GameInstance.NickName` _asawaken_game_instance_2))))

(event `SendMessage`
  (params (Message :type Text))
  ;[1 0 0] (Server) Chatting
  (bind _outactors (`GameplayStatics.GetAllActorsOfClass` "BP_MyPlayerController_C"))
  (for _array_element _outactors
    (`self.ReceiveMessage` _array_element Message)))

(event `ReqSpawnCharacter`
  (params (PawnClass :type "Pawn Class Reference") (MainWeaponSlotClass :type "Actor Class Reference") (`Upgrade Damage` :type "Float (double-precision)") (ShootingSpeed :type "Float (double-precision)") (ReloadSpeed :type Integer) (MaxAmmo :type Integer))
  ;[1 0 0] (Server) 빙의
  (bind _asbp_my_game_mode (cast `/Game/LapEscape/GameMode/BP_MyGameMode` (`GameplayStatics.GetGameMode`)))
  (bind _playerstart (`/Game/LapEscape/GameMode/BP_MyGameMode.SetPlayerStart` _asbp_my_game_mode))
  (bind _pawn (`self.SpawnCharacter` PawnClass _playerstart))
  (`self.Possess` _pawn)
  ;[1 0 0] (Server) Weapon Spawn
  (`self.WeaponSpawn` _pawn MainWeaponSlotClass `Upgrade Damage` ShootingSpeed ReloadSpeed MaxAmmo))

(event `self.ReceivePossess`
  (params (PossessedPawn :type "Pawn Object Reference"))
  ;[1 1 1] Character Rotate
  (`self.ResOnPossess` PossessedPawn))

(event `ReceiveMessage`
  (params (Message :type Text))
  ;[1 1 1] Chat Multicast
  (`/Game/LapEscape/Widget/ChatWidget/ChattingWidget.UpdateChat` (`self.ChattingWidget`) Message))

(event `InputAction|Chat`
  (params (Key :type "Key Structure"))
  ;[1 1 1] Enter로도 채팅 입력 가능
  (:`Pressed`
    (if (not (`Widget.HasKeyboardFocus` (`/Game/LapEscape/Widget/ChatWidget/ChattingWidget.EditableText_chat` (`self.ChattingWidget`))))
      (`Widget.SetKeyboardFocus` (`/Game/LapEscape/Widget/ChatWidget/ChattingWidget.EditableText_chat` (`self.ChattingWidget`))))))

(event `ResOnPossess`
  (params (NewParam :type "Pawn Object Reference"))
  ;[1 1 1] Character Rotate
  (`self.EventDispatcher_Rotate`))

(event `WeaponSpawn`
  (params (Pawn :type "Pawn Object Reference") (MainWeaponSlotClass :type "Actor Class Reference") (`Upgrade Damage` :type "Float (double-precision)") (ShootingSpeed :type "Float (double-precision)") (ReloadSpeed :type Integer) (MaxAmmo :type Integer))
  ;[1 0 0] (Server) Weapon Spawn
  (bind _returnvalue (`GameplayStatics.GetCurrentLevelName` true))
  (if (`KismetStringLibrary.NotEqual_StrStr` _returnvalue "RepairShop1")
    (bind _asbp_mixamo_character (cast `/Game/LapEscape/GameMode/BP_MixamoCharacter` Pawn))
    (`self.Weapon_TravelLevel` MainWeaponSlotClass `Upgrade Damage` ShootingSpeed ReloadSpeed MaxAmmo _asbp_mixamo_character)))

(event `Add_to_Player_List`
  (params (Player :type "Character Object Reference (by ref)"))
  (`KismetArrayLibrary.Array_Add` (`self.Player_List`) Player))

(fn `SpawnCharacter`
  (params (PawnClass :type "Pawn Class Reference") (PlayerStart :type "Actor Object Reference"))
  (returns (Pawn :type "Pawn Object Reference"))
  (bind _returnvalue (`|SpawnActorFromClass` PawnClass (`KismetMathLibrary.MakeTransform` (`self.K2_GetActorLocation` PlayerStart)) "Undefined" "OverrideRootScale" null null))
  (return _returnvalue))

(fn `UserConstructionScript`)

(fn `Weapon_TravelLevel`
  (params (MainWeaponSlotClass :type "Actor Class Reference") (`Upgrade Damage` :type "Float (double-precision)") (ShootingSpeed :type "Float (double-precision)") (ReloadSpeed :type Integer) (MaxAmmo :type Integer) (Character :type "/Game/LapEscape/GameMode/BP_MixamoCharacter Object Reference"))
  (returns (`Attached Actor` :type "Actor Object Reference"))
  (locals (MainWeaponSlotClass_Local :type "Actor Class Reference") (UpgradeDamage_Local :type "Float (double-precision)") (ShootingSpeed_Local :type "Float (double-precision)") (ReloadSpeed_Local :type Integer) (MaxAmmo_Local :type Integer) (Character_Local :type "/Game/LapEscape/GameMode/BP_MixamoCharacter Object Reference"))
  (bind _character_local (`local.Character_Local`))
  (bind _upgradedamage_local (`local.UpgradeDamage_Local`))
  (bind _reloadspeed_local (`local.ReloadSpeed_Local`))
  (bind _maxammo_local (`local.MaxAmmo_Local`))
  (bind _character_local_2 (`local.Character_Local`))
  (bind _character_local_3 (`local.Character_Local`))
  (bind _shootingspeed_local (`local.ShootingSpeed_Local`))
  (`|ExecutionSequence`
    (:`then_0`
      (set `local.MainWeaponSlotClass_Local` MainWeaponSlotClass))
    (:`then_1`
      (set `local.UpgradeDamage_Local` `Upgrade Damage`))
    (:`then_2`
      (set `local.ShootingSpeed_Local` ShootingSpeed))
    (:`then_3`
      (set `local.ReloadSpeed_Local` ReloadSpeed))
    (:`then_4`
      (set `local.MaxAmmo_Local` MaxAmmo))
    (:`then_5`
      (set `local.Character_Local` Character))
    (:`then_6`
      (bind _returnvalue (`|SpawnActorFromClass` "/Game/LapEscape/Blueprints/Weapon/BP_Pistol.BP_Pistol_C" (`KismetMathLibrary.MakeTransform` (0.0 0.0 0.0)) "Undefined" "OverrideRootScale" self "Pistol" (`local.ShootingSpeed_Local`) (`local.UpgradeDamage_Local`) (`local.ReloadSpeed_Local`) (`local.MaxAmmo_Local`) null))
      (message `/Game/LapEscape/Blueprints/Weapon/BPI_Weapon.Attach` _returnvalue _character_local)
      (set `/Game/LapEscape/GameMode/BP_MixamoCharacter.AttachedActor` _returnvalue _character_local)
      (set `/Game/LapEscape/GameMode/BP_MixamoCharacter.SubWeaponSlot` _returnvalue _character_local)
      (if (== (`local.MainWeaponSlotClass_Local`) "/Game/LapEscape/Blueprints/Weapon/BP_Rifle.BP_Rifle_C")
        (bind _returnvalue_2 (`|SpawnActorFromClass` "/Game/LapEscape/Blueprints/Weapon/BP_Rifle.BP_Rifle_C" (`KismetMathLibrary.MakeTransform` (0.0 0.0 0.0)) "Undefined" "OverrideRootScale" self "None" _shootingspeed_local _upgradedamage_local _reloadspeed_local _maxammo_local null))
        (message `/Game/LapEscape/Blueprints/Weapon/BPI_Weapon.Attach` _returnvalue_2 _character_local_2)
        (set `/Game/LapEscape/GameMode/BP_MixamoCharacter.AttachedActor` _returnvalue_2 _character_local_2)
        (bind _output_get (set `/Game/LapEscape/GameMode/BP_MixamoCharacter.MainWeaponSlot` _returnvalue_2 _character_local_2))
        (return _output_get)
        (else
          (bind _returnvalue_3 (`|SpawnActorFromClass` "/Game/LapEscape/Blueprints/Weapon/BP_Shotgun.BP_Shotgun_C" (`KismetMathLibrary.MakeTransform` (0.0 0.0 0.0)) "Undefined" "OverrideRootScale" self "None" _shootingspeed_local _upgradedamage_local _reloadspeed_local _maxammo_local null))
          (message `/Game/LapEscape/Blueprints/Weapon/BPI_Weapon.Attach` _returnvalue_3 _character_local_3)
          (set `/Game/LapEscape/GameMode/BP_MixamoCharacter.AttachedActor` _returnvalue_3 _character_local_3)
          (bind _output_get_2 (set `/Game/LapEscape/GameMode/BP_MixamoCharacter.MainWeaponSlot` _returnvalue_3 _character_local_3))
          (return _output_get_2))))))