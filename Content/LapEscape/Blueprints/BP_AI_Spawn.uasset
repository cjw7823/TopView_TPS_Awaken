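; BP_AI_Spawn is a LapEscape spawner Blueprint that links the player character's AI spawn dispatcher to a defence start event.
; On BeginPlay it binds to BP_MixamoCharacter's dispatcher, retrying by timer until the cast succeeds.
; A request/response event pair currently only prints "Start".
; SpawnAI creates a man and a woman AI at the actor's location, but no graph here calls it.
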(event `self.ReceiveBeginPlay`
  (`self.BindDispach`))

(event `ReqDefence_Start`
  (`self.ResDefence_Start`))

(event `ResDefence_Start`
  (`KismetSystemLibrary.PrintString` "Start" true true (struct :`R` 1.0 :`G` 0.014468 :`A` 1.0)))

(fn `BindDispach`
  (bind _asbp_mixamo_character (cast `/Game/LapEscape/GameMode/BP_MixamoCharacter` (`GameplayStatics.GetPlayerCharacter` 0))
    (:`then`
      (add `/Game/LapEscape/GameMode/BP_MixamoCharacter.EventDispatcher_AI_Spawn` _asbp_mixamo_character (`|CreateDelegate` :!event `BP_AI_Spawn_AutoGenFunc`)))
    (:`CastFailed`
      (`KismetSystemLibrary.K2_SetTimer` null "BindDispach" 0.1))))

(fn `BP_AI_Spawn_AutoGenFunc`
  (`self.ReqDefence_Start`))

(fn `Spawn_AI`
  (`|SpawnActorFromClass` "/Game/LapEscape/AI/BP_AI_Man.BP_AI_Man_C" (`KismetMathLibrary.MakeTransform` (`self.K2_GetActorLocation`)) "Undefined" "OverrideRootScale" null null)
  (`|SpawnActorFromClass` "/Game/LapEscape/AI/BP_AI_Woman.BP_AI_Woman_C" (`KismetMathLibrary.MakeTransform` (`self.K2_GetActorLocation`)) "Undefined" "OverrideRootScale" null null))

(fn `UserConstructionScript`)