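; Soldier character Blueprint whose skill, tied to the HUD's SteamPack widget, grants a temporary walk speed boost.
; ResSkill runs Haste immediately and on a looping one-second timer, provided the widget is not marked used.
; Haste raises the PlayerState's custom speed once, applies it to CharacterMovement and shows a particle effect.
; When the tick count reaches the PlayerState's maximum, it clears the timer, reverses the multiplier and hides the effect.
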(event `self.ResSkill`
  ;[1 1 1] Soldier Skill
  (bind _asbp_my_hud (cast `/Game/LapEscape/GameMode/BP_MyHUD` (`PlayerController.GetHUD` (`GameplayStatics.GetPlayerController` 0))))
  (if (not (`/Game/LapEscape/Widget/SkillWidget/SkillWidgetSteamPack.IsUsed` (`/Game/LapEscape/Widget/MasterWidget/InGameMasterWidget.SkillWidgetSteamPack` (`/Game/LapEscape/GameMode/BP_MyHUD.InGameMasterWidget` _asbp_my_hud))))
    (`self.Haste`)
    (`KismetSystemLibrary.K2_SetTimer` null "Haste" 1.0 true)))

(fn `Haste`
  (bind _asbp_my_player_state (cast `/Game/LapEscape/GameMode/BP_MyPlayerState` (`self.PlayerState`)))
  (if (< (`self.SkillCountTick`) (`/Game/LapEscape/GameMode/BP_MyPlayerState.MaxSkillTick` _asbp_my_player_state))
    (`/Engine/EditorBlueprintResources/StandardMacros.IncrementInt` (`self.SkillCountTick`)
      (:`  `
        (`KismetSystemLibrary.PrintString` "이속 증가" true true (struct :`G` 0.66 :`B` 1.0 :`A` 1.0) 10.0)
        (if (not (`self.OnSkill`))
          (bind _asbp_my_player_state_2 (cast `/Game/LapEscape/GameMode/BP_MyPlayerState` (`self.PlayerState`)))
          (bind _output_get (set `/Game/LapEscape/GameMode/BP_MyPlayerState.MaxWalkSpeed(custom)` (* (`/Game/LapEscape/GameMode/BP_MyPlayerState.MaxWalkSpeed(custom)` _asbp_my_player_state_2) 1.5) _asbp_my_player_state_2))
          (set `CharacterMovementComponent.MaxWalkSpeed` _output_get (`self.CharacterMovement`))
          (set `self.OnSkill` true)
          (`SceneComponent.SetVisibility` (`self.ParticleSystem`) true false))))
    (else
      (`KismetSystemLibrary.K2_ClearTimer` null "Haste")
      (bind _asbp_my_player_state_3 (cast `/Game/LapEscape/GameMode/BP_MyPlayerState` (`self.PlayerState`)))
      (bind _output_get_2 (set `/Game/LapEscape/GameMode/BP_MyPlayerState.MaxWalkSpeed(custom)` (/ (* (`/Game/LapEscape/GameMode/BP_MyPlayerState.MaxWalkSpeed(custom)` _asbp_my_player_state_3) 2.0) 3.0) _asbp_my_player_state_3))
      (set `CharacterMovementComponent.MaxWalkSpeed` _output_get_2 (`self.CharacterMovement`))
      (set `self.SkillCountTick` 0)
      (`KismetSystemLibrary.PrintString` "스킬 종료")
      (set `self.OnSkill` false)
      (`SceneComponent.SetVisibility` (`self.ParticleSystem`) false false))))

(fn `UserConstructionScript`
  (`parent.UserConstructionScript`))