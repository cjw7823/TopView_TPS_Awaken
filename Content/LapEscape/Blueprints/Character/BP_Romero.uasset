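; BP_Romero is a character Blueprint whose passive skill grants extra bonus gold.
; On BeginPlay it shows an on-screen passive-skill message, then raises BonusGold on BP_MyGameState by a fixed amount.
; It copies the new total into Awaken_GameInstance, stopping early if either cast fails.
; The construction script only calls the parent.
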(event `self.ReceiveBeginPlay`
  (`KismetSystemLibrary.PrintString` "패시브 스킬 사용중" true true (struct :`R` 0.996759 :`G` 1.0 :`A` 1.0) 60.0)
  (bind _asbp_my_game_state (cast `/Game/LapEscape/GameMode/BP_MyGameState` (`GameplayStatics.GetGameState`)))
  (bind _output_get (set `/Game/LapEscape/GameMode/BP_MyGameState.BonusGold` (+ (`/Game/LapEscape/GameMode/BP_MyGameState.BonusGold` _asbp_my_game_state) 5) _asbp_my_game_state))
  (bind _asawaken_game_instance (cast `/Game/LapEscape/Awaken_GameInstance` (`GameplayStatics.GetGameInstance`)))
  (set `/Game/LapEscape/Awaken_GameInstance.BonusGold` _output_get _asawaken_game_instance))

(fn `UserConstructionScript`
  (`parent.UserConstructionScript`))