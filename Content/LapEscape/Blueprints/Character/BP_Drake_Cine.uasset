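; BP_Drake_Cine is the Drake character Blueprint, implementing a heal-over-time skill.
; ResSkill checks that the HUD's heal skill widget is not used, then calls DoHealing immediately and on a looping one-second timer.
; Each tick heals a tenth of max HP through BP_MyPlayerState, attaches a particle effect to the mesh and prints debug HP.
; At the player state's tick limit, it clears the timer and resets the counter.
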(event `self.ResSkill`
  ;[1 1 1] Drake Skill
  (bind _asbp_my_hud (cast `/Game/LapEscape/GameMode/BP_MyHUD` (`PlayerController.GetHUD` (`GameplayStatics.GetPlayerController` 0))))
  (if (not (`/Game/LapEscape/Widget/SkillWidget/SkillWidgetHeal.IsUsed` (`/Game/LapEscape/Widget/MasterWidget/InGameMasterWidget.SkillWidgetHeal` (`/Game/LapEscape/GameMode/BP_MyHUD.InGameMasterWidget` _asbp_my_hud))))
    (`self.DoHealing`)
    (`KismetSystemLibrary.K2_SetTimer` null "DoHealing" 1.0 true)))

(fn `DoHealing`
  (bind _asbp_my_player_state (cast `/Game/LapEscape/GameMode/BP_MyPlayerState` (`self.PlayerState`)))
  (if (< (`self.SkillCountTick`) (`/Game/LapEscape/GameMode/BP_MyPlayerState.MaxSkillTick` _asbp_my_player_state))
    (bind _asbp_my_player_state_2 (cast `/Game/LapEscape/GameMode/BP_MyPlayerState` (`self.PlayerState`)))
    (`/Game/LapEscape/GameMode/BP_MyPlayerState.HealHP` _asbp_my_player_state_2 (/ (`/Game/LapEscape/GameMode/BP_MyPlayerState.MaxHP` _asbp_my_player_state_2) 10.0))
    (`/Engine/EditorBlueprintResources/StandardMacros.IncrementInt` (`self.SkillCountTick`)
      (:`  `
        (bind _asbp_my_player_state_3 (cast `/Game/LapEscape/GameMode/BP_MyPlayerState` (`self.PlayerState`)))
        (`KismetSystemLibrary.PrintString` (`KismetStringLibrary.Conv_DoubleToString` (`/Game/LapEscape/GameMode/BP_MyPlayerState.CurHP` _asbp_my_player_state_3)) true true (struct :`G` 0.66 :`B` 1.0 :`A` 1.0) 10.0)
        (`GameplayStatics.SpawnEmitterAttached` "/Game/Particle/P_DrakeSkill.P_DrakeSkill" (`self.Mesh`) "None" (0.0 0.0 0.0) (struct) (1.5 1.5 1.5))))
    (else
      (`KismetSystemLibrary.K2_ClearTimer` null "DoHealing")
      (`KismetSystemLibrary.PrintString` "스킬 종료" true true (struct :`G` 0.66 :`B` 1.0 :`A` 1.0) 5.0)
      (set `self.SkillCountTick` 0))))

(fn `UserConstructionScript`
  (`parent.UserConstructionScript`))