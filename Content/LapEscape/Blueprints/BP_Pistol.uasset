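; BP_Pistol is a weapon Blueprint that initializes as "Pistol" and handles trigger pulls with a short aim-angle animation.
; PullTriger offsets RotationXRoll on the owner's Escaper_AnimBP, then plays the shoot montage and repeats it at the weapon data's ShootSpeed interval.
; A fast looping PistolShoot timer steps the angle back up, clearing itself once it passes zero.
; The montage timer is not cleared in this Blueprint.
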(event `self.ReceiveBeginPlay`
  (bind _output_get (set `self.WeaponName` "Pistol"))
  (`self.Initialize` _output_get))

(fn `PistolShoot`
  (bind _asescaper_anim_bp (cast `/Game/Mannequin/Escaper_AnimBP` (`SkeletalMeshComponent.GetAnimInstance` (`Character.Mesh` (`self.Own Char`)))))
  (bind _rotation_x__roll_ (`/Game/Mannequin/Escaper_AnimBP.Rotation X (Roll)` _asescaper_anim_bp))
  (set `/Game/Mannequin/Escaper_AnimBP.Rotation X (Roll)` (+ _rotation_x__roll_ 1.0) _asescaper_anim_bp)
  (if (> _rotation_x__roll_ 0.0)
    (`KismetSystemLibrary.K2_ClearTimer` null "PistolShoot")))

(fn `PullTriger`
  (params (Character :type "Character Object Reference"))
  (returns (Result :type Boolean))
  ;[1 1 1] Pistol Shoot 각도 초기화
  (bind _asescaper_anim_bp (cast `/Game/Mannequin/Escaper_AnimBP` (`SkeletalMeshComponent.GetAnimInstance` (`Character.Mesh` (`self.Own Char`)))))
  (set `/Game/Mannequin/Escaper_AnimBP.Rotation X (Roll)` -4.0 _asescaper_anim_bp)
  ;[1 1 1] Pistol Shoot 각도 조절
  (`KismetSystemLibrary.K2_SetTimer` null "PistolShoot" 0.01 true)
  (`self.PlayShootMontage`)
  (`KismetSystemLibrary.K2_SetTimer` null "PlayShootMontage" (`.ShootSpeed_34_4E288DC84ACABE581897F28268AFB570` (break `/Game/LapEscape/Data/ST_Weapon` (`self.Weapon Data`))) true)
  (return false))

(fn `UserConstructionScript`
  (`parent.UserConstructionScript`))