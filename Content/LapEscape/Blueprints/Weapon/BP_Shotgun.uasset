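; BP_Shotgun is the shotgun weapon, a child Blueprint that initializes itself by weapon name at BeginPlay.
; Its shoot montage step extends the parent's by playing a shooting-and-reload montage on the owning character.
; HitProcess approximates spread with a short, horizontal multi-object box trace along the weapon's forward vector, excluding the owner.
; It requests damage on every hit returned and leaves trace debug drawing enabled.
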(event `self.ReceiveBeginPlay`
  (bind _output_get (set `self.WeaponName` "Shotgun"))
  (`self.Initialize` _output_get))

(fn `HitProcess`
  (bind (_returnvalue_x _returnvalue_y) (`KismetMathLibrary.BreakVector` (`self.GetActorForwardVector`)))
  (bind _returnvalue (`self.K2_GetActorLocation`))
  (bind (_outhits _returnvalue_2) (`KismetSystemLibrary.BoxTraceMultiForObjects` _returnvalue (+ _returnvalue (* (`KismetMathLibrary.MakeVector` _returnvalue_x _returnvalue_y) 400.0)) (60.0 60.0 30.0) (struct) (`|MakeArray` "ObjectTypeQuery1" "ObjectTypeQuery2" "ObjectTypeQuery3" "ObjectTypeQuery4" "ObjectTypeQuery6" :!type "EObjectTypeQuery Enum") false (`|MakeArray` (`self.Own Char`) :!type "Actor Object Reference") "ForDuration"))
  (if _returnvalue_2
    (for _array_element _outhits
      (`self.ReqApplyDamage` (`.HitActor` (`GameplayStatics.BreakHitResult` _array_element)) 2.0 (`Pawn.GetController` (`self.Own Char`)) self))))

(fn `PlayShootMontage`
  (locals (InPlayRate :type "Float (double-precision)" :default 1.0))
  (bind _own_char (`self.Own Char`))
  (`parent.PlayShootMontage`)
  (`/Engine/EditorBlueprintResources/StandardMacros.IsValid` _own_char
    (:`Is Valid`
      (`AnimInstance.Montage_Play` (`SkeletalMeshComponent.GetAnimInstance` (`Character.Mesh` _own_char)) "/Game/Mannequin/MixamoAnim/Shotgun_ShootingReload_Montage.Shotgun_ShootingReload_Montage" 1.0 "MontageLength" 0.0 false))))

(fn `UserConstructionScript`
  (`parent.UserConstructionScript`))