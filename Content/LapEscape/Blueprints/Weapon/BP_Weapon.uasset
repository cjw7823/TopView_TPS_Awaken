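; BP_Weapon is a weapon actor, configured from DT_Weapon_Mixamo, that snaps to a character's pistol socket and drops with physics on detach.
; Pulling the trigger loops the shoot montage on a timer shortened by a speedup event, skipping shots while dodging.
; DoShoot plays sound and muzzle effect; only for player pawn 0 does it spend ammo and run a horizontal line trace, routing damage through ReqApplyDamage, commented as server-side.
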(event `ReqShootingSpeedup`
  (set `self.ShootingSpeed` (+ (`self.ShootingSpeed`) 0.05)))

(event `ReqApplyDamage`
  (params (DamagedActor :type "Actor Object Reference (by ref)") (BaseDamage :type "Float (double-precision)") (EventInstigator :type "Controller Object Reference (by ref)") (DamageCauser :type "Actor Object Reference (by ref)") (`Hit Location` :type "Vector Structure") (`Impulse Dir` :type "Vector Structure"))
  ;[1 0 0] (Server)Damage
  (`GameplayStatics.ApplyDamage` DamagedActor BaseDamage EventInstigator DamageCauser))

(fn `Attach`
  (params (OwnChar :type "Character Object Reference"))
  (returns (Result :type Boolean))
  (bind _staticmesh (`self.StaticMesh`))
  (set `self.Own Char` OwnChar)
  (`PrimitiveComponent.SetSimulatePhysics` _staticmesh false)
  (`PrimitiveComponent.SetCollisionEnabled` _staticmesh "NoCollision")
  (`self.K2_AttachToComponent` (`Character.Mesh` (`self.Own Char`)) "Socket_Pistol" "SnapToTarget" "SnapToTarget" "KeepRelative")
  (bind _asbp_mixamo_character (cast `/Game/LapEscape/GameMode/BP_MixamoCharacter` (`self.Own Char`)))
  (set `/Game/LapEscape/GameMode/BP_MixamoCharacter.Type_Weapon` (`.Type_25_7807464E4B1535A814F454809CF8F6F8` (break `/Game/LapEscape/Data/ST_Weapon` (`self.Weapon Data`))) _asbp_mixamo_character)
  (return true))

(fn `Detach`
  (params (OwnChar :type "Character Object Reference"))
  (returns (Result :type Boolean))
  (bind _staticmesh (`self.StaticMesh`))
  (`self.SetOwner` null)
  (set `self.Own Char` null)
  (`SceneComponent.K2_DetachFromComponent` (`self.StaticMesh`) "KeepWorld" "KeepWorld" "KeepRelative" true)
  (`PrimitiveComponent.SetSimulatePhysics` _staticmesh true)
  (`PrimitiveComponent.SetCollisionEnabled` _staticmesh "QueryAndPhysics")
  (return true))

(fn `Do Shoot`
  (`self.SoundAndEmitter`)
  ;[1 1 1] 소유한 폰에서 히트처리
  (if (== (`self.Own Char`) (`GameplayStatics.GetPlayerPawn` 0))
    (`self.HitProcess`)
    (`KismetSystemLibrary.PrintString` "(Client)ReqApplyDamage" false true (struct :`G` 0.66 :`B` 1.0 :`A` 1.0) 20.0)
    (`/Engine/EditorBlueprintResources/StandardMacros.DecrementInt` (`self.CurAmmo`))))

(fn `HitProcess`
  (bind (_returnvalue_x _returnvalue_y) (`KismetMathLibrary.BreakVector` (`self.GetActorForwardVector`)))
  (bind _returnvalue (`self.K2_GetActorLocation`))
  (bind (_outhit _returnvalue_2) (`KismetSystemLibrary.LineTraceSingleForObjects` _returnvalue (+ _returnvalue (* (`KismetMathLibrary.MakeVector` _returnvalue_x _returnvalue_y) 2000.0)) (`|MakeArray` "ObjectTypeQuery1" "ObjectTypeQuery2" "ObjectTypeQuery3" "ObjectTypeQuery4" "ObjectTypeQuery6" :!type "EObjectTypeQuery Enum") false (`|MakeArray` (`self.Own Char`) :!type "Actor Object Reference") "ForDuration"))
  (if _returnvalue_2
    (`self.ReqApplyDamage` (`.HitActor` (`GameplayStatics.BreakHitResult` _outhit)) 10.0 (`Pawn.GetController` (`self.Own Char`)) self)))

(fn `Initialize`
  (params (WeaponName :type Name))
  (bind _returnvalue (`|GetDataTableRow` "/Game/LapEscape/Data/DT_Weapon_Mixamo.DT_Weapon_Mixamo" WeaponName)
    (:`then`
      (bind _output_get (set `self.Weapon Data` _returnvalue))
      (`|ExecutionSequence`
        (:`then_0`
          (bind (_type _staticmesh _socketname _shootspeed _shootsound _reloadsound _ammo) (break `/Game/LapEscape/Data/ST_Weapon` _output_get))
          (`StaticMeshComponent.SetStaticMesh` (`self.StaticMesh`) _staticmesh))
        (:`then_1`
          (set `self.Socket Name` _socketname))
        (:`then_2`
          (set `self.CurAmmo` _ammo))))))

(fn `PlayShootMontage`
  (bind _own_char (`self.Own Char`))
  (bind _asbp_mixamo_character (cast `/Game/LapEscape/GameMode/BP_MixamoCharacter` (`self.Own Char`)))
  (if (`/Game/LapEscape/GameMode/BP_MixamoCharacter.NotDodge` _asbp_mixamo_character)
    (`/Engine/EditorBlueprintResources/StandardMacros.IsValid` _own_char
      (:`Is Valid`
        (`AnimInstance.Montage_Play` (`SkeletalMeshComponent.GetAnimInstance` (`Character.Mesh` _own_char)) (`.ShootMontage_19_DDD868924B5E92985549DB86287CEF02` (break `/Game/LapEscape/Data/ST_Weapon` (`self.Weapon Data`))) 1.0 "MontageLength" 0.0 true)))))

(fn `PullTriger`
  (params (Character :type "Character Object Reference"))
  (returns (Result :type Boolean))
  (`self.PlayShootMontage`)
  (`KismetSystemLibrary.K2_SetTimer` null "PlayShootMontage" (- (`.ShootSpeed_34_4E288DC84ACABE581897F28268AFB570` (break `/Game/LapEscape/Data/ST_Weapon` (`self.Weapon Data`))) (`self.ShootingSpeed`)) true)
  (return false))

(fn `ReleaseTriger`
  (params (Character :type "Character Object Reference"))
  (returns (Result :type Boolean))
  (`KismetSystemLibrary.K2_ClearTimer` null "PlayShootMontage")
  (return false))

(fn `SoundAndEmitter`
  (bind _audio (`self.Audio`))
  (`AudioComponent.SetSound` _audio (`.ShootSound_10_C23006E8436552887B136BAAFF99430E` (break `/Game/LapEscape/Data/ST_Weapon` (`self.Weapon Data`))))
  (`AudioComponent.Play` _audio 0.0)
  (`GameplayStatics.SpawnEmitterAtLocation` "/Game/StarterContent/Particles/P_Explosion.P_Explosion" (`SceneComponent.GetSocketLocation` (`self.StaticMesh`) "Muzzle") (struct) (0.05 0.05 0.05)))

(fn `UserConstructionScript`)