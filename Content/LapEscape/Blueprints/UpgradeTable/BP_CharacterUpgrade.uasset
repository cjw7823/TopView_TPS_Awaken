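; BP_CharacterUpgrade is a proximity trigger that opens the character upgrade UI for a player.
; Sphere begin and end overlaps with BP_MixamoCharacter pass its controller to show and hide events.
; These toggle the existing upgrade widget in the HUD's master widget, swapping cursor widget, mouse cursor and input mode.
; Casts to the player controller and its HUD gate the change, intended to affect only that client.
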(event `HideUpgradeWidget`
  (params (CharacterController :type "Controller Object Reference"))
  ;[1 1 1] 해당 클라이언트에만 위젯 생성
  (bind _asbp_my_player_controller (cast `/Game/LapEscape/GameMode/BP_MyPlayerController` CharacterController))
  (set `PlayerController.bShowMouseCursor` false _asbp_my_player_controller)
  (bind _asbp_my_hud (cast `/Game/LapEscape/GameMode/BP_MyHUD` (`PlayerController.GetHUD` _asbp_my_player_controller)))
  (`Widget.SetVisibility` (`/Game/LapEscape/Widget/MasterWidget/InGameMasterWidget.CharacterUpgradeWidget` (`/Game/LapEscape/GameMode/BP_MyHUD.InGameMasterWidget` _asbp_my_hud)) "Collapsed")
  (`Widget.SetVisibility` (`/Game/LapEscape/GameMode/BP_MyHUD.CursorWidget` _asbp_my_hud) "Visible")
  (`WidgetBlueprintLibrary.SetInputMode_GameOnly` _asbp_my_player_controller))

(event `ShowUpgradeWidget`
  (params (CharacterConteroller :type "Controller Object Reference"))
  ;[1 1 1] 해당 클라이언트에만 위젯 생성
  (bind _asbp_my_player_controller (cast `/Game/LapEscape/GameMode/BP_MyPlayerController` CharacterConteroller))
  (set `PlayerController.bShowMouseCursor` true _asbp_my_player_controller)
  (bind _asbp_my_hud (cast `/Game/LapEscape/GameMode/BP_MyHUD` (`PlayerController.GetHUD` _asbp_my_player_controller)))
  (bind _characterupgradewidget (`/Game/LapEscape/Widget/MasterWidget/InGameMasterWidget.CharacterUpgradeWidget` (`/Game/LapEscape/GameMode/BP_MyHUD.InGameMasterWidget` _asbp_my_hud)))
  (`Widget.SetVisibility` _characterupgradewidget "Visible")
  (`Widget.SetVisibility` (`/Game/LapEscape/GameMode/BP_MyHUD.CursorWidget` _asbp_my_hud) "Collapsed")
  (`WidgetBlueprintLibrary.SetInputMode_GameAndUIEx` _asbp_my_player_controller _characterupgradewidget))

(event `self.Sphere.OnComponentBeginOverlap`
  (params (OverlappedComponent :type "PrimitiveComponent Object Reference") (OtherActor :type "Actor Object Reference") (OtherComp :type "PrimitiveComponent Object Reference") (OtherBodyIndex :type Integer) (bFromSweep :type Boolean) (SweepResult :type "HitResult Structure (by ref)"))
  ;[1 1 1] Overlap Event
  (bind _asbp_mixamo_character (cast `/Game/LapEscape/GameMode/BP_MixamoCharacter` OtherActor))
  (`self.ShowUpgradeWidget` (`Pawn.GetController` _asbp_mixamo_character)))

(event `self.Sphere.OnComponentEndOverlap`
  (params (OverlappedComponent :type "PrimitiveComponent Object Reference") (OtherActor :type "Actor Object Reference") (OtherComp :type "PrimitiveComponent Object Reference") (OtherBodyIndex :type Integer))
  ;[1 1 1] Overlap Event
  (bind _asbp_mixamo_character (cast `/Game/LapEscape/GameMode/BP_MixamoCharacter` OtherActor))
  (`self.HideUpgradeWidget` (`Pawn.GetController` _asbp_mixamo_character)))

(fn `UserConstructionScript`)