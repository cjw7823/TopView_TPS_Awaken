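; BP_Shotgun is the shotgun weapon Blueprint, a child of a parent weapon class that supplies the shared logic.
; On BeginPlay it sets WeaponName to "Shotgun" and passes it to Initialize.
; Its PlayShootMontage override calls the parent, then plays a test reload montage on the owning character's mesh, if that character is valid, without stopping other montages.
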(event `self.ReceiveBeginPlay`
  (bind _output_get (set `self.WeaponName` "Shotgun"))
  (`self.Initialize` _output_get))

(fn `PlayShootMontage`
  (bind _own_char (`self.Own Char`))
  (`parent.PlayShootMontage`)
  (`/Engine/EditorBlueprintResources/StandardMacros.IsValid` _own_char
    (:`Is Valid`
      (`AnimInstance.Montage_Play` (`SkeletalMeshComponent.GetAnimInstance` (`Character.Mesh` _own_char)) "/Game/Mannequin/RifleAnimsetPro/Animations/InPlace/Shotgun_Reload_test_Montage.Shotgun_Reload_test_Montage" 1.0 "MontageLength" 0.0 false))))

(fn `UserConstructionScript`
  (`parent.UserConstructionScript`))