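; Level travel trigger for Chapter 1 that moves the multiplayer session to the RepairShop2 map once at least two players stand inside it.
; Begin and end overlaps with BP_MixamoCharacter actors raise and lower a player count.
; When an entry brings the count to two or more, it runs a servertravel console command with the map name hardcoded.
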(event `self.ReceiveActorBeginOverlap`
  (params (OtherActor :type "Actor Object Reference"))
  (cast `/Game/LapEscape/GameMode/BP_MixamoCharacter` OtherActor)
  (`/Engine/EditorBlueprintResources/StandardMacros.IncrementInt` (`self.PlayerCount`)
    (:`  `
      (if (>= (`self.PlayerCount`) 2)
        (`KismetSystemLibrary.ExecuteConsoleCommand` "servertravel RepairShop2" null)))))

(event `self.ReceiveActorEndOverlap`
  (params (OtherActor :type "Actor Object Reference"))
  (cast `/Game/LapEscape/GameMode/BP_MixamoCharacter` OtherActor)
  (`/Engine/EditorBlueprintResources/StandardMacros.DecrementInt` (`self.PlayerCount`)))

(fn `UserConstructionScript`)